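; Base enemy actor Blueprint that can be selected by touch and killed by damage.
; A touch on the actor casts the game mode to TopDownGameMode and passes itself to EnemySelected.
; ReceiveDamage subtracts an integer amount from HP and destroys the actor at zero or below.
; The Destroy function, construction script and other events are empty.
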(event EventActorOnInputTouchBegin
  (params (FingerIndex :type ETouchIndex%20Enum :default "Touch1"))
  (bind _astop_down_game_mode (Utilities|Casting|CastToTopDownGameMode (Game|GetGameMode)))
  (Default|EnemySelected _astop_down_game_mode self))

(event EventBeginPlay)

(event Collision|EventActorBeginOverlap
  (params (OtherActor :type Actor%20Object%20Reference)))

(event EventTick
  (params (DeltaSeconds :type Float%20%28single-precision%29)))

(fn ConstructionScript)

(fn ReceiveDamage
  (params (Integer :type Integer))
  (bind _output_get (Variables|Default|SetHP (- (Variables|Default|GetHP) Integer)))
  (if (<= _output_get 0)
    (Actor|DestroyActor)))

(fn Destroy)