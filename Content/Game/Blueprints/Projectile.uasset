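; Homing projectile actor, fired by either side, that chases a Target and deals damage on overlap.
; Each tick it moves SphereMesh straight toward the Target at MoveSpeed without sweeping, and destroys itself if the Target becomes invalid.
; IsEnemyProjectile filters hits: player shots damage the overlapped BaseEnemy, while enemy shots hitting a TopDownCharacter apply damage to that character's SelectedEnemy.
; Either valid hit destroys the projectile.
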(event EventBeginPlay)

(event EventTick
  (params (DeltaSeconds :type Float%20%28single-precision%29))
  (bind _spheremesh (Variables|Default|GetSphereMesh))
  (bind _returnvalue (Transformation|GetWorldTransform _spheremesh))
  (bind (_location _rotation _scale) (Math|Transform|BreakTransform _returnvalue))
  ;[1 1 1] Moving torwads the target
  (Utilities|IsValid (Variables|Default|GetTarget)
    (:Is%20Valid
      (Transformation|SetWorldTransform (Variables|Default|GetSphereMesh) (Math|Transform|MakeTransform (+ (* (Math|Vector|Normalize (- (.Location (Math|Transform|BreakTransform (Transformation|GetWorldTransform (Variables|/Game/Game/Blueprints/Enemies/BaseEnemy.BaseEnemy_C|GetDefaultSceneRoot (Variables|Default|GetTarget))))) _location)) (* (Utilities|Time|GetWorldDeltaSeconds) (Variables|Default|GetMoveSpeed))) _location) _rotation _scale) false))
    (:Is%20Not%20Valid
      (Actor|DestroyActor))))

(event Collision|EventActorBeginOverlap
  (params (OtherActor :type Actor%20Object%20Reference))
  ;[1 1 1] Deal damage when overlapping
  (bind _asbase_enemy (Utilities|Casting|CastToBaseEnemy OtherActor)
    (:then
      (if (not (Variables|Default|GetIsEnemyProjectile))
        (Default|ReceiveDamage _asbase_enemy (Variables|Default|GetDamage))
        (Actor|DestroyActor :!label _label)))
    (:CastFailed
      (bind _astop_down_character (Utilities|Casting|CastToTopDownCharacter OtherActor))
      (if (Variables|Default|GetIsEnemyProjectile)
        (Default|ReceiveDamage (Variables|/Game/Game/Blueprints/TopDownCharacter.TopDownCharacter_C|GetSelectedEnemy _astop_down_character) (Variables|Default|GetDamage))
        (goto _label)))))

(fn ConstructionScript)